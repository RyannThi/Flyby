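; BP_Quest is the base quest Blueprint, which builds and starts a quest's objectives when play begins.
; BeginPlay constructs the root objective collection, stores it, populates it, then activates it.
; The construct and populate functions are placeholders for child classes to override, printing red errors if the base versions run.
; A getter exposes the stored root collection.
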(event EventBeginPlay
  (bind _rootobjcolection (Private|ConstructRootObjectiveCollection))
  (bind _output_get (Variables|Private|SetRootObjectiveCollection _rootobjcolection))
  (Private|PopulateObjectives _output_get)
  (Default|ActivateObjective (Variables|Private|GetRootObjectiveCollection)))

(fn ConstructionScript)

(fn ConstructRootObjectiveCollection
  (Development|PrintString "ERROR:createRootColection called for base class " true true "(R=1.000000,G=0.000000,B=0.043376,A=1.000000)")
  (return 0))

(fn PopulateObjectives
  (params (RootObjCollection :type BP%20Obj%20Collection%20Object%20Reference))
  (Development|PrintString "ERROR:PopulateObjectives called for base class " true true "(R=1.000000,G=0.000000,B=0.043376,A=1.000000)"))

(fn GetRootObjectiveCollection
  (return (Variables|Private|GetRootObjectiveCollection)))