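; BP_Quest_01 defines the "Delivery supplies" quest, in which three islands must be reached in order.
; It builds a root BP_ObjCollection with order required, then fills it with three BP_ObjReachDestination objectives.
; Each objective takes its own island trigger as destination and is added in island sequence.
; The construction script only calls its parent.
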(fn ConstructionScript
  (|CallParentFunction))

(fn ConstructRootObjectiveCollection
  (bind _returnvalue (Game|ConstructObjectfromClass "/Game/BP/QuestSystem/Objective/BP_ObjCollection.BP_ObjCollection_C" self true "Delivery supplies"))
  (return _returnvalue))

(fn PopulateObjectives
  (params (RootObjCollection :type BP%20Obj%20Collection%20Object%20Reference))
  (Utilities|FlowControl|Sequence
    (:then_0
      (bind _returnvalue (Game|ConstructObjectfromClass "/Game/BP/QuestSystem/Objective/BP_ObjReachDestination.BP_ObjReachDestination_C" self (Variables|Default|GetFirstIslandTrigger) "Reach Island 1"))
      (Default|AddObjective RootObjCollection _returnvalue))
    (:then_1
      (bind _returnvalue_2 (Game|ConstructObjectfromClass "/Game/BP/QuestSystem/Objective/BP_ObjReachDestination.BP_ObjReachDestination_C" self (Variables|Default|GetSecondIslandTrigger) "Reach Island 2"))
      (Default|AddObjective RootObjCollection _returnvalue_2))
    (:then_2
      (bind _returnvalue_3 (Game|ConstructObjectfromClass "/Game/BP/QuestSystem/Objective/BP_ObjReachDestination.BP_ObjReachDestination_C" self (Variables|Default|GetThirdIslandTrigger) "Reach Island 3"))
      (Default|AddObjective RootObjCollection _returnvalue_3))))